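; Footstep anim notify that plays surface-specific sound and Niagara effects for BP_ArcoroxCharacter.
; It asks the owning character for its surface type and picks a sound and particle system for metal, stone, tile, grass or water.
; Both spawn at the BoneName socket on the mesh, with ShouldPlaySound gating only the audio.
; Unlisted surfaces leave the sound and effect variables unchanged.
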(fn ReceivedNotify
  (params (MeshComp :type Skeletal%20Mesh%20Component%20Object%20Reference) (Animation :type Anim%20Sequence%20Base%20Object%20Reference) (EventReference :type Anim%20Notify%20Event%20Reference%20Structure%20%28by%20ref%29))
  (bind _bonename (Variables|Default|GetBoneName))
  (bind _returnvalue (Transformation|GetSocketLocation MeshComp _bonename))
  (bind _asbp_arcorox_character (Utilities|Casting|CastToBP_ArcoroxCharacter (Components|GetOwner MeshComp)))
  (bind _returnvalue_2 (Class|ArcoroxCharacter|GetSurfaceType _asbp_arcorox_character))
  (switch Utilities|FlowControl|Switch|SwitchonEPhysicalSurface _returnvalue_2
    (:SurfaceType_Default
      _)
    (:SurfaceType1
      (LocalVariables|SetFootstepSound "/Game/Static/Assets/Sounds/MetaSounds/Footsteps/SFX_MetalFootstep.SFX_MetalFootstep")
      (LocalVariables|SetFootstepNiagaraSystem "/Game/Static/AssetPacks/A_Surface_Footstep/Niagara_FX/ParticleSystems/PSN_General1_Surface.PSN_General1_Surface"))
    (:SurfaceType2
      (LocalVariables|SetFootstepSound "/Game/Static/Assets/Sounds/MetaSounds/Footsteps/SFX_StoneFootstep.SFX_StoneFootstep")
      (LocalVariables|SetFootstepNiagaraSystem "/Game/Static/AssetPacks/A_Surface_Footstep/Niagara_FX/ParticleSystems/PSN_Gravel_Surface.PSN_Gravel_Surface"))
    (:SurfaceType3
      (LocalVariables|SetFootstepSound "/Game/Static/Assets/Sounds/MetaSounds/Footsteps/SFX_TileFootstep.SFX_TileFootstep")
      (LocalVariables|SetFootstepNiagaraSystem "/Game/Static/AssetPacks/A_Surface_Footstep/Niagara_FX/ParticleSystems/PSN_General2_Surface.PSN_General2_Surface"))
    (:SurfaceType4
      (LocalVariables|SetFootstepSound "/Game/Static/Assets/Sounds/MetaSounds/Footsteps/SFX_GrassFootstep.SFX_GrassFootstep")
      (LocalVariables|SetFootstepNiagaraSystem "/Game/Static/AssetPacks/A_Surface_Footstep/Niagara_FX/ParticleSystems/PSN_Grass_Surface.PSN_Grass_Surface"))
    (:SurfaceType5
      (LocalVariables|SetFootstepSound "/Game/Static/Assets/Sounds/MetaSounds/Footsteps/SFX_WaterFootstep.SFX_WaterFootstep")
      (LocalVariables|SetFootstepNiagaraSystem "/Game/Static/AssetPacks/A_Surface_Footstep/Niagara_FX/ParticleSystems/PSN_WaterLight_Surface.PSN_WaterLight_Surface")))
  (if (Variables|Default|GetShouldPlaySound)
    (Audio|PlaySoundatLocation (LocalVariables|GetFootstepSound) _returnvalue "0, 0, 0" 1.0 1.0 0.0 0 0 0 0))
  (Niagara|SpawnSystematLocation (LocalVariables|GetFootstepNiagaraSystem) _returnvalue)
  (return true))