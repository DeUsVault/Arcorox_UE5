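; Anim notify that plays a surface-dependent landing sound when the Arcorox character lands from a jump.
; It casts the mesh owner to BP_ArcoroxCharacter and switches on its surface type to pick a metal, stone, tile, grass or water sound.
; The sound plays at the owner's location; unmatched surfaces leave the sound variable unchanged, and non-Arcorox owners play nothing.
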(fn ReceivedNotify
  (params (MeshComp :type Skeletal%20Mesh%20Component%20Object%20Reference) (Animation :type Anim%20Sequence%20Base%20Object%20Reference) (EventReference :type Anim%20Notify%20Event%20Reference%20Structure%20%28by%20ref%29))
  (bind _returnvalue (Components|GetOwner MeshComp))
  (bind _asbp_arcorox_character (Utilities|Casting|CastToBP_ArcoroxCharacter _returnvalue))
  (bind _returnvalue_2 (Class|ArcoroxCharacter|GetSurfaceType _asbp_arcorox_character))
  (switch Utilities|FlowControl|Switch|SwitchonEPhysicalSurface _returnvalue_2
    (:SurfaceType_Default
      _)
    (:SurfaceType1
      (LocalVariables|SetJumpLandSound "/Game/Static/Assets/Sounds/MetaSounds/JumpLand/SFX_Metal_JumpLand.SFX_Metal_JumpLand"))
    (:SurfaceType2
      (LocalVariables|SetJumpLandSound "/Game/Static/Assets/Sounds/MetaSounds/JumpLand/SFX_Stone_JumpLand.SFX_Stone_JumpLand"))
    (:SurfaceType3
      (LocalVariables|SetJumpLandSound "/Game/Static/Assets/Sounds/MetaSounds/JumpLand/SFX_Tile_JumpLand.SFX_Tile_JumpLand"))
    (:SurfaceType4
      (LocalVariables|SetJumpLandSound "/Game/Static/Assets/Sounds/MetaSounds/JumpLand/SFX_Grass_JumpLand.SFX_Grass_JumpLand"))
    (:SurfaceType5
      (LocalVariables|SetJumpLandSound "/Game/Static/Assets/Sounds/MetaSounds/JumpLand/SFX_Water_JumpLand.SFX_Water_JumpLand")))
  (Audio|PlaySoundatLocation (LocalVariables|GetJumpLandSound) (Transformation|GetActorLocation _returnvalue) "0, 0, 0" 1.0 1.0 0.0 0 0 0 0)
  (return true))